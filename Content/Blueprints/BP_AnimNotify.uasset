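; Anim notify that plays a surface-dependent footstep sound during animations.
; When triggered, it line traces down from the owning actor on the Visibility channel, with persistent debug drawing.
; The hit's physical surface selects a concrete, wood or dirt sound, with dirt as the fallback.
; The sound plays at the world origin rather than at the actor or hit point.
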(fn ReceivedNotify
  (params (MeshComp :type Skeletal%20Mesh%20Component%20Object%20Reference) (Animation :type Anim%20Sequence%20Base%20Object%20Reference) (EventReference :type Anim%20Notify%20Event%20Reference%20Structure%20%28by%20ref%29))
  (bind _returnvalue (Components|GetOwner MeshComp))
  (bind _returnvalue_2 (Transformation|GetActorLocation _returnvalue))
  (bind (_outhit _returnvalue_3) (Collision|LineTraceByChannel _returnvalue_2 (+ _returnvalue_2 (* (Transformation|GetActorUpVector _returnvalue) -2e+02)) "TraceTypeQuery1" false 0 "Persistent"))
  (if _returnvalue_3
    (switch Utilities|FlowControl|Switch|SwitchonEPhysicalSurface (Collision|GetSurfaceType _outhit)
      (:SurfaceType_Default
        (Audio|PlaySoundatLocation "/Game/Audio/FootSteps/MS_FT_Dirt.MS_FT_Dirt" "0, 0, 0" "0, 0, 0" 1.0 1.0 0.0 0 0 0 0 :!label _label))
      (:SurfaceType1
        (Audio|PlaySoundatLocation "/Game/Audio/FootSteps/MS_FT_Concrete.MS_FT_Concrete" "0, 0, 0" "0, 0, 0" 1.0 1.0 0.0 0 0 0 0))
      (:SurfaceType2
        (goto _label))
      (:SurfaceType3
        (Audio|PlaySoundatLocation "/Game/Audio/FootSteps/MS_FT_Wood.MS_FT_Wood" "0, 0, 0" "0, 0, 0" 1.0 1.0 0.0 0 0 0 0))))
  (return false))